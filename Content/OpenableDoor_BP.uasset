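; OpenableDoor_BP is a door actor that swings open and closed through OpenDoor open and close request events.
; The DoorOpening timeline plays or reverses, adding its OpenAngle yaw to a base rotation and playing Explosion01 at the door on its Sound Timing event.
; The base rotation derives from InitialRotation, which despite its name stores the actor's starting location, converted with RotationFromXVector.
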(event `self.ReceiveBeginPlay`
  (set `self.InitialRotation` (`self.K2_GetActorLocation`)))

(event `self.OpenDoor.OpenDoorRequest`
  (bind (_direction _openangle) (`Timeline|Door Opening` :!label _label)
    (:`Update`
      (`self.SetActorRotation` (`KismetMathLibrary.ComposeRotators` (`KismetMathLibrary.MakeRotator` 0.0 0.0 _openangle) (`KismetMathLibrary.Conv_VectorToRotator` (`self.InitialRotation`)))))
    (:`SoundTiming`
      (`GameplayStatics.PlaySoundAtLocation` "/Game/StarterContent/Audio/Explosion01.Explosion01" (`self.K2_GetActorLocation`)))))

(event `self.OpenDoor.CloseDoorRequest`
  (goto _label :!via `Reverse`))

(fn `UserConstructionScript`)